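; BP_AnomalyChair is an anomaly rocking chair actor that spins in the level until it is cleared.
; Every tick, the RockingChairA mesh rotates steadily around yaw.
; Calling Clear stops the spin, shrinks the chair linearly toward zero scale over about five seconds, then destroys the actor after a matching delay.
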(event EventBeginPlay
  (Variables|Default|SetScale 1.0))

(event Collision|EventActorBeginOverlap
  (params (OtherActor :type Actor%20Object%20Reference)))

(event EventTick
  (params (DeltaSeconds :type Float%20%28single-precision%29))
  (if (and (Variables|Default|GetClearing) (> (Variables|Default|GetScale) 0.0))
    (bind _output_get (Variables|Default|SetScale (- (Variables|Default|GetScale) (* DeltaSeconds 0.2))))
    (Transformation|SetRelativeScale3D (Variables|Default|GetRockingChair_a) (Math|Vector|MakeVector _output_get _output_get _output_get))
    (else
      (Transformation|AddWorldRotation (Variables|Default|GetRockingChair_a) (Math|Rotator|MakeRotator 0.0 0.0 (* DeltaSeconds 6e+01)) false false))))

(event EventClear
  (Variables|Default|SetClearing true)
  (Utilities|FlowControl|Delay 5.0)
  (Actor|DestroyActor))

(fn ConstructionScript)