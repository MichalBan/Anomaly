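; BP_StartPawn is a pawn in the Start folder that slowly rolls its camera around the view axis.
; On BeginPlay it picks a random spin direction and starts a looping timer that periodically reverses it.
; Tick applies a frame-rate-independent roll to the Camera, scaled by the current sign.
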(event EventBeginPlay
  (if (Math|Random|RandomBool)
    (Variables|Default|SetSignum 1.0)
    (else
      (Variables|Default|SetSignum -1.0)))
  (Utilities|Time|SetTimerbyFunctionName 0 "ChangeDirection" 12.0 true))

(event Collision|EventActorBeginOverlap
  (params (OtherActor :type Actor%20Object%20Reference)))

(event EventTick
  (params (DeltaSeconds :type Float%20%28single-precision%29))
  (Transformation|AddLocalRotation (Variables|Default|GetCamera) (Math|Rotator|MakeRotator (* DeltaSeconds 3e+01 (Variables|Default|GetSignum)) 0.0 0.0) false false))

(fn ConstructionScript)

(fn ChangeDirection
  (Variables|Default|SetSignum (* (Variables|Default|GetSignum) -1.0)))