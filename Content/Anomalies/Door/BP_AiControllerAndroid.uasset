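; AI controller for the Android in the Door anomaly folder, running BehaviorTreeAndroid on possession.
; AI perception writes a sensed Player-tagged actor to the blackboard as EnemyActor and sets CanSee.
; Any other perception update starts a SightTimer delay that then clears both keys.
; A renewed player sighting does not cancel that pending timer.
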(event OnTargetPerceptionUpdated(AIPerception)
  (params (Actor :type Actor%20Object%20Reference) (Stimulus :type AI%20Stimulus%20Structure))
  (bind _returnvalue (AI|GetBlackboard 0))
  (if (and (Actor|ActorHasTag Actor "Player") (Utilities|Struct|BreakAIStimulus Stimulus))
    (Utilities|IsValid _returnvalue
      (:Is%20Valid
        (AI|Components|Blackboard|SetValueasBool _returnvalue (Variables|Default|GetCanSee) true)
        (AI|Components|Blackboard|SetValueasObject _returnvalue (Variables|Default|GetEnemyActor) Actor)))
    (else
      (bind _returnvalue_2 (Utilities|Time|SetTimerbyEvent (delegate Custom|StartEnemyTimer) (Variables|Default|GetSightTimer)))
      (Variables|Default|SetEnemyTimer _returnvalue_2))))

(event Custom|StartEnemyTimer
  (bind _returnvalue (AI|GetBlackboard 0))
  (if (Utilities|IsValid _returnvalue)
    (AI|Components|Blackboard|SetValueasBool _returnvalue (Variables|Default|GetCanSee) false)
    (AI|Components|Blackboard|SetValueasObject _returnvalue (Variables|Default|GetEnemyActor) 0)))

(event EventBeginPlay)

(event EventTick
  (params (DeltaSeconds :type Float%20%28single-precision%29)))

(event EventPossess
  (params (PossessedPawn :type Pawn%20Object%20Reference))
  (AI|RunBehaviorTree "/Game/Anomalies/Door/BehaviorTreeAndroid.BehaviorTreeAndroid"))

(fn ConstructionScript)