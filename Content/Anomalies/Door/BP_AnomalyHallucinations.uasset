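; Door anomaly that plays hallucination footage on the player's HUD and erodes sanity at close range.
; Activation opens the media source at a random time; closing hides the image and closes the player.
; While active, Tick uses player distance to toggle the HUD image and, within a slightly wider radius, drain sanity over time.
; Overlapping its box also deals a one-off sanity hit, without checking the active state.
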(event OnComponentBeginOverlap(Box)
  (params (OverlappedComponent :type Primitive%20Component%20Object%20Reference) (OtherActor :type Actor%20Object%20Reference) (OtherComp :type Primitive%20Component%20Object%20Reference) (OtherBodyIndex :type Integer) (bFromSweep :type Boolean) (SweepResult :type Hit%20Result%20Structure%20%28by%20ref%29))
  (bind _asbp_first_person_character (Utilities|Casting|CastToBP_FirstPersonCharacter OtherActor))
  (Class|AnomalyCharacter|ChangeSanity _asbp_first_person_character -1.0))

(event EventBeginPlay
  (Media|MediaPlayer|Close (Variables|Default|GetMediaPlayer) :!class /Script/MediaAssets.MediaPlayer))

(event Collision|EventActorBeginOverlap
  (params (OtherActor :type Actor%20Object%20Reference)))

(event EventTick
  (params (DeltaSeconds :type Float%20%28single-precision%29))
  (bind _returnvalue (Game|Player|GetPlayerPawn 0))
  (bind _returnvalue_2 (Transformation|GetActorLocation))
  (bind _returnvalue_3 (Transformation|GetActorLocation _returnvalue))
  (bind _returnvalue_4 (Math|Vector|Distance(Vector) _returnvalue_3 _returnvalue_2))
  (if (Variables|Default|GetbActive)
    (CallFunction|ShowHallucinations (< _returnvalue_4 2e+02))
    (if (< _returnvalue_4 3e+02)
      (bind _asanomaly_character (Utilities|Casting|CastToAnomalyCharacter (Game|Player|GetPlayerPawn 0)))
      (Class|AnomalyCharacter|ChangeSanity _asanomaly_character (* DeltaSeconds (Variables|Default|GetSanityDrain) -1.0)))))

(event EventActivateAnomaly
  (Media|MediaPlayer|OpenSource (Variables|Default|GetMediaPlayer) "/Game/Movies/Hallucinations.Hallucinations")
  (Media|MediaPlayer|Seek (Variables|Default|GetMediaPlayer) (Math|Timespan|MakeTimespan 0 0 0 (Math|Random|RandomInteger 120))))

(event EventClear)

(event EventOnClose
  (CallFunction|ShowHallucinations false)
  (Media|MediaPlayer|Close (Variables|Default|GetMediaPlayer) :!class /Script/MediaAssets.MediaPlayer))

(fn ConstructionScript)

(fn ShowHallucinations
  (params (Show :type Boolean))
  (bind _asanomaly_player_controller (Utilities|Casting|CastToAnomalyPlayerController (Game|GetPlayerController 0)))
  (bind _asbp_hudwidget (Utilities|Casting|CastToBP_HUDWidget (Class|AnomalyPlayerController|GetHUDWidget _asanomaly_player_controller)))
  (if Show
    (Widget|SetVisibility (Variables|/Game/HUD/BP_HUDWidget.BP_HUDWidget_C|GetImage_hallucination _asbp_hudwidget) "Visible")
    (else
      (Widget|SetVisibility (Variables|/Game/HUD/BP_HUDWidget.BP_HUDWidget_C|GetImage_hallucination _asbp_hudwidget) "Hidden"))))