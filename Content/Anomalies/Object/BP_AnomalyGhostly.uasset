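; Anomaly actor that turns an assigned object into a ghostly version that can drain player sanity.
; Setup swaps the object's material for a dynamic ghost material, keeping its BaseColor texture.
; Tick fades audio up when the camera is near and facing it, down otherwise, draining sanity whenever VolumeMultiplier equals the target volume.
; Clear flashes the material white and opaque, then destroys the object and itself after delays.
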(event EventBeginPlay
  (Utilities|IsValid (Variables|Default|GetModel)
    (:Is%20Valid
      (Actor|SetOwner (Variables|Default|GetModel) self)
      (bind _returnvalue (Rendering|Material|CreateDynamicMaterialInstance (Rendering|Material|GetMaterial (Variables|/Script/Engine.StaticMeshActor|GetStaticMeshComponent (Variables|Default|GetModel)) 0) "None" "None" :!class /Script/Engine.KismetMaterialLibrary))
      (bind _returnvalue_2 (Rendering|Material|GetTextureParameterValue _returnvalue "BaseColor" :!class /Script/Engine.MaterialInstanceDynamic))
      (bind _returnvalue_3 (Rendering|Material|CreateDynamicMaterialInstance "/Game/Anomalies/Object/GhostlyMaterial.GhostlyMaterial" "None" "None" :!class /Script/Engine.KismetMaterialLibrary))
      (Rendering|Material|SetTextureParameterValue _returnvalue_3 "BaseColor" _returnvalue_2)
      (Rendering|Material|SetMaterial (Variables|/Script/Engine.StaticMeshActor|GetStaticMeshComponent (Variables|Default|GetModel)) 0 _returnvalue_3))))

(event Collision|EventActorBeginOverlap
  (params (OtherActor :type Actor%20Object%20Reference)))

(event EventTick
  (params (DeltaSeconds :type Float%20%28single-precision%29))
  (bind _returnvalue (Game|GetPlayerController 0))
  (bind _model (Variables|Default|GetModel))
  (bind _returnvalue_2 (Transformation|GetActorLocation _model))
  (bind _playercameramanager (Variables|/Script/Engine.PlayerController|GetPlayerCameraManager _returnvalue))
  (bind _returnvalue_3 (Camera|GetCameraLocation _playercameramanager))
  (bind _returnvalue_4 (- _returnvalue_2 _returnvalue_3))
  (Utilities|IsValid (Variables|Default|GetModel)
    (:Is%20Valid
      (if (and (< (Math|Vector|VectorLength _returnvalue_4) 5e+02) (< (Class|KismetMathLibrary|DegAcos (Math|Vector|DotProduct (Math|Vector|Normalize _returnvalue_4) (Math|Vector|GetForwardVector (Camera|GetCameraRotation _playercameramanager)))) 3e+01))
        (Variables|Default|SetVolume 1.0)
        (else
          (Variables|Default|SetVolume 0.01)))
      (Audio|Components|Audio|AdjustVolume (Variables|Default|GetAudioComponent) (Variables|Default|GetSanityDelay) (Variables|Default|GetVolume) "Linear" :!class /Script/Engine.AudioComponent)
      (if (== (Variables|/Script/Engine.AudioComponent|GetVolumeMultiplier (Variables|Default|GetAudioComponent)) (Variables|Default|GetVolume))
        (bind _asanomaly_character (Utilities|Casting|CastToAnomalyCharacter (Game|Player|GetPlayerPawn 0)))
        (Class|AnomalyCharacter|ChangeSanity _asanomaly_character (* DeltaSeconds (Variables|Default|GetSanityDrain) -1.0))))))

(event EventClear
  (Utilities|FlowControl|Delay 0.2)
  (bind _asmaterial_instance_dynamic (Utilities|Casting|CastToMaterialInstanceDynamic (Rendering|Material|GetMaterial (Variables|/Script/Engine.StaticMeshActor|GetStaticMeshComponent (Variables|Default|GetModel)) 0)))
  (Rendering|Material|SetVectorParameterValue _asmaterial_instance_dynamic "EmissiveColor" "(R=1.000000,G=1.000000,B=1.000000,A=1.000000)" :!class /Script/Engine.MaterialInstanceDynamic)
  (Rendering|Material|SetScalarParameterValue _asmaterial_instance_dynamic "Opacity" 1.0 :!class /Script/Engine.MaterialInstanceDynamic)
  (Utilities|FlowControl|Delay 0.3)
  (Actor|DestroyActor (Variables|Default|GetModel))
  (Utilities|FlowControl|Delay 1.0)
  (Actor|DestroyActor))

(event EventSetObject
  (params (Object :type Static%20Mesh%20Actor%20Object%20Reference))
  (Variables|Default|SetModel Object)
  (Actor|SetOwner (Variables|Default|GetModel) self)
  (bind _returnvalue (Rendering|Material|CreateDynamicMaterialInstance (Rendering|Material|GetMaterial (Variables|/Script/Engine.StaticMeshActor|GetStaticMeshComponent (Variables|Default|GetModel)) 0) "None" "None" :!class /Script/Engine.KismetMaterialLibrary))
  (bind _returnvalue_2 (Rendering|Material|GetTextureParameterValue _returnvalue "BaseColor" :!class /Script/Engine.MaterialInstanceDynamic))
  (bind _returnvalue_3 (Rendering|Material|CreateDynamicMaterialInstance "/Game/Anomalies/Object/GhostlyMaterial.GhostlyMaterial" "None" "None" :!class /Script/Engine.KismetMaterialLibrary))
  (Rendering|Material|SetTextureParameterValue _returnvalue_3 "BaseColor" _returnvalue_2)
  (Rendering|Material|SetMaterial (Variables|/Script/Engine.StaticMeshActor|GetStaticMeshComponent (Variables|Default|GetModel)) 0 _returnvalue_3))

(fn ConstructionScript)