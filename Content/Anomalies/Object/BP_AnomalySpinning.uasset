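; BP_AnomalySpinning is an anomaly actor that spins an assigned object and drains the player's sanity.
; SetObject or BeginPlay makes the Model movable, attaches it to the anomaly and takes ownership.
; Tick yaws the model and reduces AnomalyCharacter sanity by SanityDrain over time.
; Once cleared, the model shrinks and rises instead, and the Clear event destroys both actors after a delay.
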(event EventBeginPlay
  (bind _model (Variables|Default|GetModel))
  (Variables|Default|SetScale 1.0)
  (Utilities|IsValid _model
    (:Is%20Valid
      (Transformation|SetMobility _model "Movable")
      (Transformation|AttachComponentToComponent _model (Variables|Default|GetDefaultSceneRoot) "None" "SnapToTarget" "KeepWorld" "SnapToTarget" true)
      (Actor|SetOwner (Variables|Default|GetModel) self))))

(event Collision|EventActorBeginOverlap
  (params (OtherActor :type Actor%20Object%20Reference)))

(event EventTick
  (params (DeltaSeconds :type Float%20%28single-precision%29))
  (bind _model (Variables|Default|GetModel))
  (bind _rootcomponent (Variables|/Script/Engine.Actor|GetRootComponent _model))
  (Utilities|IsValid (Variables|Default|GetModel)
    (:Is%20Valid
      (if (and (Variables|Default|GetbClear) (> (Variables|Default|GetScale) 0.0))
        (bind _output_get (Variables|Default|SetScale (- (Variables|Default|GetScale) (* DeltaSeconds 0.2))))
        (Transformation|SetRelativeScale3D _rootcomponent (Math|Vector|MakeVector _output_get _output_get _output_get))
        (Transformation|AddWorldOffset _rootcomponent (Math|Vector|MakeVector 0.0 0.0 (* 1e+01 DeltaSeconds)) false false)
        (else
          (Transformation|AddWorldRotation (Variables|/Script/Engine.Actor|GetRootComponent (Variables|Default|GetModel)) (Math|Rotator|MakeRotator 0.0 0.0 (* DeltaSeconds 6e+01)) false false)
          (bind _asanomaly_character (Utilities|Casting|CastToAnomalyCharacter (Game|Player|GetPlayerPawn 0)))
          (Class|AnomalyCharacter|ChangeSanity _asanomaly_character (* DeltaSeconds (Variables|Default|GetSanityDrain) -1.0)))))))

(event EventClear
  (Utilities|FlowControl|Delay 5.0)
  (Actor|DestroyActor (Variables|Default|GetModel))
  (Actor|DestroyActor))

(event EventSetObject
  (params (Object :type Static%20Mesh%20Actor%20Object%20Reference))
  (Variables|Default|SetModel Object)
  (Transformation|SetMobility (Variables|Default|GetModel) "Movable")
  (Transformation|AttachComponentToComponent (Variables|Default|GetModel) (Variables|Default|GetDefaultSceneRoot) "None" "SnapToTarget" "KeepWorld" "SnapToTarget" true)
  (Actor|SetOwner (Variables|Default|GetModel) self))

(fn ConstructionScript)