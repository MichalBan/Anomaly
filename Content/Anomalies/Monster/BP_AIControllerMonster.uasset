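; AI controller for the monster anomaly that, five seconds after possessing a BP_CharacterMonster, sets it to killing and runs its behavior tree.
; Successfully sensing a player-tagged actor cancels the sight timer and writes CanSee and EnemyActor to the blackboard.
; Any other perception update starts a timer that clears both keys when it expires.
; SetCleared sets a separate blackboard bool to true.
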(event OnTargetPerceptionUpdated(AIPerception)
  (params (Actor :type Actor%20Object%20Reference) (Stimulus :type AI%20Stimulus%20Structure))
  (bind _returnvalue (AI|GetBlackboard 0))
  (if (and (Actor|ActorHasTag Actor "Player") (Utilities|Struct|BreakAIStimulus Stimulus))
    (Utilities|Time|ClearandInvalidateTimerbyHandle (Variables|Default|GetEnemyTimer))
    (Utilities|IsValid _returnvalue
      (:Is%20Valid
        (AI|Components|Blackboard|SetValueasBool _returnvalue (Variables|Default|GetCanSee) true)
        (AI|Components|Blackboard|SetValueasObject _returnvalue (Variables|Default|GetEnemyActor) Actor)))
    (else
      (bind _returnvalue_2 (Utilities|Time|SetTimerbyEvent (delegate Custom|StartEnemyTimer) (Variables|Default|GetSightTimer)))
      (Variables|Default|SetEnemyTimer _returnvalue_2))))

(event Custom|StartEnemyTimer
  (bind _returnvalue (AI|GetBlackboard 0))
  (AI|Components|Blackboard|SetValueasBool _returnvalue (Variables|Default|GetCanSee) false)
  (AI|Components|Blackboard|SetValueasObject _returnvalue (Variables|Default|GetEnemyActor) 0))

(event EventBeginPlay)

(event EventTick
  (params (DeltaSeconds :type Float%20%28single-precision%29)))

(event EventPossess
  (params (PossessedPawn :type Pawn%20Object%20Reference))
  (bind _asbp_character_monster (Utilities|Casting|CastToBP_CharacterMonster PossessedPawn))
  (Utilities|FlowControl|Delay 5.0)
  (Variables|/Game/Anomalies/Monster/BP_CharacterMonster.BP_CharacterMonster_C|SetKilling _asbp_character_monster true)
  (AI|RunBehaviorTree "/Game/Anomalies/Monster/BehaviorTreeMonster.BehaviorTreeMonster"))

(fn ConstructionScript)

(fn SetCleared
  (bind _returnvalue (AI|GetBlackboard 0))
  (Utilities|IsValid _returnvalue
    (:Is%20Valid
      (AI|Components|Blackboard|SetValueasBool _returnvalue (LocalVariables|GetKey) true))))