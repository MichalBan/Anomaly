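; BP_AnomalyMonster is the monster anomaly actor, wrapping a monster character in a child actor component.
; On BeginPlay it spawns a BP_AIControllerMonster at the child's transform, possesses the child pawn and becomes its owner.
; Clear flags both character and controller as cleared, then destroys the monster and itself after a short delay.
; The Tick branch on Clear does nothing.
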(event EventBeginPlay
  (bind _bp_charactermonster (Variables|Default|GetBP_CharacterMonster))
  (bind _childactor (Variables|/Script/Engine.ChildActorComponent|GetChildActor _bp_charactermonster))
  (bind _returnvalue (Game|SpawnActorfromClass "/Game/Anomalies/Monster/BP_AIControllerMonster.BP_AIControllerMonster_C" (Transformation|GetActorTransform _childactor) "AlwaysSpawn" "MultiplyWithRoot" 0 0))
  (bind _aspawn (Utilities|Casting|CastToPawn _childactor))
  (Pawn|Possess _returnvalue _aspawn)
  (Actor|SetOwner _aspawn self))

(event Collision|EventActorBeginOverlap
  (params (OtherActor :type Actor%20Object%20Reference)))

(event EventTick
  (params (DeltaSeconds :type Float%20%28single-precision%29))
  (if (Variables|Default|GetbClear)
    _))

(event EventClear
  (bind _asbp_character_monster (Utilities|Casting|CastToBP_CharacterMonster (Variables|/Script/Engine.ChildActorComponent|GetChildActor (Variables|Default|GetBP_CharacterMonster))))
  (Variables|/Game/Anomalies/Monster/BP_CharacterMonster.BP_CharacterMonster_C|SetCleared _asbp_character_monster true)
  (bind _asbp_aicontroller_monster (Utilities|Casting|CastToBP_AIControllerMonster (Pawn|GetController _asbp_character_monster)))
  (Default|SetCleared _asbp_aicontroller_monster)
  (Utilities|FlowControl|Delay 4.0)
  (Actor|DestroyActor (Variables|/Script/Engine.ChildActorComponent|GetChildActor (Variables|Default|GetBP_CharacterMonster)))
  (Actor|DestroyActor))

(fn ConstructionScript)