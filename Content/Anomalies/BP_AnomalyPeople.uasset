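; Anomaly actor that opens a door and plays hallucination media when activated, until it is cleared.
; ActivateAnomaly starts the media and a looping timer that keeps seeking to random timestamps, while Tick swings the referenced Door actor open.
; While active, player proximity shows the HUD hallucination image and raises MediaSound volume.
; Clear swings the door back, then Tick hides the image, stops media and timer, and destroys the actor.
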(event Custom|Seek
  (Media|MediaPlayer|Seek (Variables|Default|GetMediaPlayer) (Math|Timespan|MakeTimespan 0 0 0 (Math|Random|RandomInteger 9999))))

(event EventBeginPlay)

(event Collision|EventActorBeginOverlap
  (params (OtherActor :type Actor%20Object%20Reference)))

(event EventTick
  (params (DeltaSeconds :type Float%20%28single-precision%29))
  (bind _returnvalue (* DeltaSeconds 3e+01))
  (bind _returnvalue_2 (* _returnvalue -1.0))
  (if (Variables|Default|GetAnomalyActive)
    (bind _asanomaly_hud (Utilities|Casting|CastToAnomalyHUD (HUD|GetHUD (Game|GetPlayerController 0))))
    (bind _asbp_hudwidget (Utilities|Casting|CastToBP_HUDWidget (Class|AnomalyHUD|GetHUDWidget _asanomaly_hud)))
    (if (> (Math|Vector|Distance(Vector) (Transformation|GetActorLocation (Game|Player|GetPlayerPawn 0)) (Transformation|GetActorLocation)) 2e+02)
      (Widget|SetVisibility (Variables|/Game/HUD/BP_HUDWidget.BP_HUDWidget_C|GetImage_hallucination _asbp_hudwidget) "Hidden")
      (Audio|Components|Audio|SetVolumeMultiplier (Variables|Default|GetMediaSound) 0.1 :!class /Script/AudioMixer.SynthComponent :!label _label)
      (else
        (Widget|SetVisibility (Variables|/Game/HUD/BP_HUDWidget.BP_HUDWidget_C|GetImage_hallucination _asbp_hudwidget) "Visible")
        (Audio|Components|Audio|SetVolumeMultiplier (Variables|Default|GetMediaSound) 1.0 :!class /Script/AudioMixer.SynthComponent)))
    (else
      (goto _label)))
  (if (Variables|Default|GetDoorOpening)
    (Transformation|AddActorLocalRotation (Variables|Default|GetDoor) (Math|Rotator|MakeRotator 0.0 0.0 _returnvalue) false false)
    (bind _output_get (Variables|Default|SetDoorYaw (+ (Variables|Default|GetDoorYaw) _returnvalue)))
    (if (> _output_get 9e+01)
      (Variables|Default|SetDoorOpening false))
    (elif (Variables|Default|GetDoorClosing)
      (Transformation|AddActorLocalRotation (Variables|Default|GetDoor) (Math|Rotator|MakeRotator 0.0 0.0 _returnvalue_2) false false)
      (bind _output_get_2 (Variables|Default|SetDoorYaw (+ (Variables|Default|GetDoorYaw) _returnvalue_2)))
      (if (< _output_get_2 -9e+01)
        (Variables|Default|SetDoorClosing false)
        (bind _asanomaly_hud_2 (Utilities|Casting|CastToAnomalyHUD (HUD|GetHUD (Game|GetPlayerController 0))))
        (bind _asbp_hudwidget_2 (Utilities|Casting|CastToBP_HUDWidget (Class|AnomalyHUD|GetHUDWidget _asanomaly_hud_2)))
        (Widget|SetVisibility (Variables|/Game/HUD/BP_HUDWidget.BP_HUDWidget_C|GetImage_hallucination _asbp_hudwidget_2) "Hidden")
        (Media|MediaPlayer|Close (Variables|Default|GetMediaPlayer) :!class /Script/MediaAssets.MediaPlayer)
        (Utilities|Time|ClearandInvalidateTimerbyHandle (Variables|Default|GetSeekTimer))
        (Actor|DestroyActor)))))

(event EventActivateAnomaly
  (Variables|Default|SetAnomalyActive true)
  (Media|MediaPlayer|OpenSource (Variables|Default|GetMediaPlayer) (Variables|Default|GetMediaSource))
  (Utilities|FlowControl|Delay 0.2)
  (Media|MediaPlayer|Seek (Variables|Default|GetMediaPlayer) (Math|Timespan|MakeTimespan 0 0 0 (Math|Random|RandomInteger 9999)))
  (Variables|Default|SetDoorOpening true)
  (Variables|Default|SetDoorYaw 0.0)
  (bind _returnvalue (Utilities|Time|SetTimerbyEvent (delegate Custom|Seek) 3.0 true false 0.1))
  (Variables|Default|SetSeekTimer _returnvalue))

(event EventClear
  (Variables|Default|SetDoorClosing true)
  (Variables|Default|SetDoorYaw 0.0))

(fn ConstructionScript)